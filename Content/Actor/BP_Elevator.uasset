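; BP_Elevator is an elevator actor that, in this graph, handles a single sliding door.
; Open plays a timeline that lerps Door1 along relative X from its stored initial location.
; Close, also triggered when an overlap with the Box ends, reverses that timeline.
; An IsDoorSliding flag ignores new requests until the timeline finishes, so a Close during movement is dropped.
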(event OnComponentEndOverlap(Box)
  (params (OverlappedComponent :type Primitive%20Component%20Object%20Reference) (OtherActor :type Actor%20Object%20Reference) (OtherComp :type Primitive%20Component%20Object%20Reference) (OtherBodyIndex :type Integer))
  (bind _d1_initial_location (Variables|Default|GetD1%20Initial%20Location))
  (if (not (Variables|Default|GetIsDoorSliding?))
    (Variables|Default|SetIsDoorSliding? true)
    (bind _door1move (Timeline|时间轴D1 Reverse)
      (:Update
        (Transformation|SetRelativeLocation (Variables|Default|GetDoor1) (Math|Vector|MakeVector (Math|Float|Lerp (.x _d1_initial_location) (- (.x _d1_initial_location) -4e+02) _door1move) (.y _d1_initial_location) (.z _d1_initial_location)) false false))
      (:Finished
        (Variables|Default|SetIsDoorSliding? false)))))

(event Custom|Open
  (bind _d1_initial_location (Variables|Default|GetD1%20Initial%20Location))
  (if (not (Variables|Default|GetIsDoorSliding?))
    (Variables|Default|SetIsDoorSliding? true)
    (bind _door1move (Timeline|时间轴D1 Play)
      (:Update
        (Transformation|SetRelativeLocation (Variables|Default|GetDoor1) (Math|Vector|MakeVector (Math|Float|Lerp (.x _d1_initial_location) (- (.x _d1_initial_location) -4e+02) _door1move) (.y _d1_initial_location) (.z _d1_initial_location)) false false))
      (:Finished
        (Variables|Default|SetIsDoorSliding? false)))))

(event Custom|Close
  (bind _d1_initial_location (Variables|Default|GetD1%20Initial%20Location))
  (if (not (Variables|Default|GetIsDoorSliding?))
    (Variables|Default|SetIsDoorSliding? true)
    (bind _door1move (Timeline|时间轴D1 Reverse)
      (:Update
        (Transformation|SetRelativeLocation (Variables|Default|GetDoor1) (Math|Vector|MakeVector (Math|Float|Lerp (.x _d1_initial_location) (- (.x _d1_initial_location) -4e+02) _door1move) (.y _d1_initial_location) (.z _d1_initial_location)) false false))
      (:Finished
        (Variables|Default|SetIsDoorSliding? false)))))

(fn ConstructionScript)