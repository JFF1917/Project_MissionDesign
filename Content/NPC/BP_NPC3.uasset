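; BP_NPC3 is a dialogue NPC that can turn into an enemy soldier.
; Outside of fair mode (IsInFair), its sphere overlap gives the player dialogue input, the interact widget and the DialogueID, then removes input and widget and interrupts dialogue on exit.
; Overlap also toggles IsTalk unless it was initially true.
; BecomeEnemy replaces the NPC with an AI_Soldier at its location, yawed 90 degrees, passing on IsPazlok and IsEbenezer.
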(event OnComponentBeginOverlap(Sphere)
  (params (OverlappedComponent :type Primitive%20Component%20Object%20Reference) (OtherActor :type Actor%20Object%20Reference) (OtherComp :type Primitive%20Component%20Object%20Reference) (OtherBodyIndex :type Integer) (bFromSweep :type Boolean) (SweepResult :type Hit%20Result%20Structure%20%28by%20ref%29))
  (if (not (Variables|Default|GetIsInFair?))
    (bind _asplayer_rebel_x (Utilities|Casting|CastToPlayer_RebelX OtherActor))
    (Default|AddIMCDialogue _asplayer_rebel_x)
    (UserInterface|Viewport|AddtoViewport (Variables|/Game/RebelX_Core/Blueprints/Player_RebelX.Player_RebelX_C|GetWBP_DiaInteract_Ins _asplayer_rebel_x) 0)
    (Variables|/Game/RebelX_Core/Blueprints/Player_RebelX.Player_RebelX_C|SetDialogueID _asplayer_rebel_x (Variables|Default|GetDialogue%20ID))
    (if (not (Variables|Default|GetIsTalkInitial?))
      (Variables|Default|SetIsTalk? true))))

(event OnComponentEndOverlap(Sphere)
  (params (OverlappedComponent :type Primitive%20Component%20Object%20Reference) (OtherActor :type Actor%20Object%20Reference) (OtherComp :type Primitive%20Component%20Object%20Reference) (OtherBodyIndex :type Integer))
  (if (not (Variables|Default|GetIsInFair?))
    (bind _asplayer_rebel_x (Utilities|Casting|CastToPlayer_RebelX OtherActor))
    (Default|DeleteIMCDialogue _asplayer_rebel_x)
    (Widget|RemovefromParent (Variables|/Game/RebelX_Core/Blueprints/Player_RebelX.Player_RebelX_C|GetWBP_DiaInteract_Ins _asplayer_rebel_x))
    (Default|InteruptDialogue _asplayer_rebel_x)
    (if (not (Variables|Default|GetIsTalkInitial?))
      (Variables|Default|SetIsTalk? false))))

(event Custom|BecomeEnemy
  (bind _returnvalue (Transformation|GetActorRotation))
  (bind _returnvalue_2 (Transformation|GetActorLocation))
  (Game|SpawnActorfromClass "/Game/RebelX_Core/Blueprints/AI/_Soldier/AI_Soldier.AI_Soldier_C" (Math|Transform|MakeTransform (Math|Vector|MakeVector (.x _returnvalue_2) (.y _returnvalue_2) (.z _returnvalue_2)) (Math|Rotator|MakeRotator (.roll _returnvalue) (.pitch _returnvalue) (+ (.yaw _returnvalue) 9e+01)) "1.000000,1.000000,1.000000") "Undefined" "MultiplyWithRoot" 0 (Variables|Default|GetIs%20Pazlok?) (Variables|Default|GetIs%20Ebenezer?) 0)
  (Actor|DestroyActor))

(event EventBeginPlay
  (Variables|Default|SetDialogue%20ID (Variables|Default|GetInitialDialogueID))
  (Variables|Default|SetIsTalkInitial? (Variables|Default|GetIsTalk?)))

(fn ConstructionScript)