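; BP_SequenceTrigger plays a Level Sequence shortly after BeginPlay, apparently as a level intro; its overlap event is empty.
; It switches input to UI-only during playback, hides the RebelX HUD core and calls HideUI on the player.
; A fixed delay, rather than a sequence-finished event, then restores the HUD core and game-only input, provided the HUD core was valid.
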(event EventBeginPlay
  (bind _returnvalue (Game|GetPlayerController 0))
  (bind _returnvalue_2 (Game|GetPlayerController 0))
  (Utilities|FlowControl|Delay 0.05)
  (Variables|/Script/Engine.PlayerController|SetbShowMouseCursor _returnvalue false)
  (Input|SetInputModeUIOnly _returnvalue 0 "DoNotLock" false)
  (bind _returnvalue_3 (Sequencer|Player|CreateLevelSequencePlayer (Variables|Default|GetLevel%20Sequence) (Variables|Default|GetSettings)))
  (Sequencer|Player|Play _returnvalue_3 :!class /Script/MovieScene.MovieSceneSequencePlayer)
  (bind _ashud_rebel_x (Utilities|Casting|CastToHUD_RebelX (HUD|GetHUD (Game|GetPlayerController 0))))
  (bind _hudcore (Variables|/Game/RebelX_Core/Blueprints/HUD_RebelX.HUD_RebelX_C|GetHUDCore _ashud_rebel_x)
    (:then
      (Widget|SetVisibility _hudcore "Hidden")
      (bind _asplayer_rebel_x (Utilities|Casting|CastToPlayer_RebelX (Game|GetPlayerCharacter 0)))
      (Default|HideUI _asplayer_rebel_x)
      (Utilities|FlowControl|Delay 6.8)
      (Widget|SetVisibility _hudcore "Visible")
      (Variables|/Script/Engine.PlayerController|SetbShowMouseCursor _returnvalue_2 false)
      (Input|SetInputModeGameOnly _returnvalue_2 false))
    (:else)))

(event Collision|EventActorBeginOverlap
  (params (OtherActor :type Actor%20Object%20Reference)))

(event EventTick
  (params (DeltaSeconds :type Float%20%28single-precision%29)))

(fn ConstructionScript)