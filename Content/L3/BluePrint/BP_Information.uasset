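; BP_Information is an interactable info-copy point that advances a Player_RebelX side mission when the player holds E nearby.
; Box overlap toggles two prompt widgets and the actor's input for that player.
; While E is held, a self-calling Adding event with a one-second Delay increments the player's Info counter.
; At the threshold, a DoOnce awards a side mission point, plays a ping and checks side mission completion.
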(event OnComponentBeginOverlap(Box)
  (params (OverlappedComponent :type Primitive%20Component%20Object%20Reference) (OtherActor :type Actor%20Object%20Reference) (OtherComp :type Primitive%20Component%20Object%20Reference) (OtherBodyIndex :type Integer) (bFromSweep :type Boolean) (SweepResult :type Hit%20Result%20Structure%20%28by%20ref%29))
  (if (== OtherActor (Variables|Default|GetAs%20Player%20Rebel%20X))
    (Input|EnableInput (Game|GetPlayerController 0))
    (Rendering|SetVisibility (Variables|Default|GetWidget) true false)
    (Rendering|SetVisibility (Variables|Default|GetWidget1) true false)))

(event OnComponentEndOverlap(Box)
  (params (OverlappedComponent :type Primitive%20Component%20Object%20Reference) (OtherActor :type Actor%20Object%20Reference) (OtherComp :type Primitive%20Component%20Object%20Reference) (OtherBodyIndex :type Integer))
  (if (== OtherActor (Variables|Default|GetAs%20Player%20Rebel%20X))
    (Input|DisableInput (Game|GetPlayerController 0))
    (Rendering|SetVisibility (Variables|Default|GetWidget) false false)
    (Rendering|SetVisibility (Variables|Default|GetWidget1) false false)))

(event Custom|InfoCopyDone
  (bind _as_player_rebel_x (Variables|Default|GetAs%20Player%20Rebel%20X))
  (if (>= (Variables|/Game/RebelX_Core/Blueprints/Player_RebelX.Player_RebelX_C|GetInfo%25 (Variables|Default|GetAs%20Player%20Rebel%20X)) 3.0)
    (Utilities|FlowControl|DoOnce false
      (:Completed
        (Variables|/Game/RebelX_Core/Blueprints/Player_RebelX.Player_RebelX_C|SetSideMissionPoint _as_player_rebel_x (+ (Variables|/Game/RebelX_Core/Blueprints/Player_RebelX.Player_RebelX_C|GetSideMissionPoint _as_player_rebel_x) 1))
        (Audio|PlaySound2D "/Engine/EngineSounds/1kSineTonePing.1kSineTonePing" 1.0 1.0 0.0 0 0)
        (Default|CheckSideAllDone (Variables|Default|GetAs%20Player%20Rebel%20X))))))

(event Custom|Adding
  (bind _as_player_rebel_x (Variables|Default|GetAs%20Player%20Rebel%20X))
  (if (Variables|Default|GetIs%20adding?)
    (bind _result (Math|Float|IncrementFloat (Variables|/Game/RebelX_Core/Blueprints/Player_RebelX.Player_RebelX_C|GetInfo%25 _as_player_rebel_x))
      (:%20%20
        (Variables|/Game/RebelX_Core/Blueprints/Player_RebelX.Player_RebelX_C|SetInfo%25 _as_player_rebel_x _result)
        (Utilities|FlowControl|Delay 1.0)
        (if (Variables|Default|GetIs%20adding?)
          (CallFunction|Adding)
          (CallFunction|InfoCopyDone)
          (else
            (CallFunction|InfoCopyDone)))))))

(event EventBeginPlay
  (bind _asplayer_rebel_x (Utilities|Casting|CastToPlayer_RebelX (Game|GetPlayerCharacter 0)))
  (Variables|Default|SetAs%20Player%20Rebel%20X _asplayer_rebel_x))

(event Collision|EventActorBeginOverlap
  (params (OtherActor :type Actor%20Object%20Reference)))

(event EventTick
  (params (DeltaSeconds :type Float%20%28single-precision%29)))

(event Input|KeyboardEvents|DebugKeyE
  (params (Key :type Key%20Structure :default "None") (ActionValue :type Input%20Action%20Value%20Structure))
  (:Pressed
    (Variables|Default|SetIs%20adding? true)
    (CallFunction|Adding))
  (:Released
    (Variables|Default|SetIs%20adding? false)))

(fn ConstructionScript)