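; Level 3 trigger actor that plays the LS_02 level sequence the first time Player_RebelX overlaps its Box.
; A DoOnce gates the overlap, then a level sequence player is created and started.
; If the HUD_RebelX core widget is valid, it is hidden and HideUI2 is called on the player.
; A fixed delay, independent of sequence completion, then makes the HUD core visible again.
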(event OnComponentBeginOverlap(Box)
  (params (OverlappedComponent :type Primitive%20Component%20Object%20Reference) (OtherActor :type Actor%20Object%20Reference) (OtherComp :type Primitive%20Component%20Object%20Reference) (OtherBodyIndex :type Integer) (bFromSweep :type Boolean) (SweepResult :type Hit%20Result%20Structure%20%28by%20ref%29))
  (Utilities|Casting|CastToPlayer_RebelX OtherActor)
  (Utilities|FlowControl|DoOnce false
    (:Completed
      (bind _returnvalue (Sequencer|Player|CreateLevelSequencePlayer "/Game/L3/LevelSequence/LS_02.LS_02" (Variables|Default|GetSettings)))
      (Sequencer|Player|Play _returnvalue :!class /Script/MovieScene.MovieSceneSequencePlayer)
      (bind _ashud_rebel_x (Utilities|Casting|CastToHUD_RebelX (HUD|GetHUD (Game|GetPlayerController 0))))
      (bind _hudcore (Variables|/Game/RebelX_Core/Blueprints/HUD_RebelX.HUD_RebelX_C|GetHUDCore _ashud_rebel_x)
        (:then
          (Widget|SetVisibility _hudcore "Hidden")
          (bind _asplayer_rebel_x (Utilities|Casting|CastToPlayer_RebelX (Game|GetPlayerCharacter 0)))
          (Default|HideUI2 _asplayer_rebel_x)
          (Utilities|FlowControl|Delay 4.3)
          (Widget|SetVisibility _hudcore "Visible"))
        (:else)))))

(event EventBeginPlay)

(event Collision|EventActorBeginOverlap
  (params (OtherActor :type Actor%20Object%20Reference)))

(event EventTick
  (params (DeltaSeconds :type Float%20%28single-precision%29)))

(fn ConstructionScript)