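; Lockable puzzle wall that damages overlapping Characters and sinks out of the way once unlocked.
; A looping timer applies damage to every overlapping Character, starting on Box overlap and clearing when none remain.
; Unlock adds to a lock count; on reaching the required total, a timeline lowers the actor and level sequence LS_03 plays, once.
; Box1 toggles the actor's input for Player_RebelX, though no input events are defined here.
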(event OnComponentBeginOverlap(Box1)
  (params (OverlappedComponent :type Primitive%20Component%20Object%20Reference) (OtherActor :type Actor%20Object%20Reference) (OtherComp :type Primitive%20Component%20Object%20Reference) (OtherBodyIndex :type Integer) (bFromSweep :type Boolean) (SweepResult :type Hit%20Result%20Structure%20%28by%20ref%29))
  (Utilities|Casting|CastToPlayer_RebelX OtherActor)
  (Input|EnableInput (Game|GetPlayerController 0)))

(event OnComponentEndOverlap(Box1)
  (params (OverlappedComponent :type Primitive%20Component%20Object%20Reference) (OtherActor :type Actor%20Object%20Reference) (OtherComp :type Primitive%20Component%20Object%20Reference) (OtherBodyIndex :type Integer))
  (Utilities|Casting|CastToPlayer_RebelX OtherActor)
  (Input|DisableInput (Game|GetPlayerController 0)))

(event OnComponentBeginOverlap(Box)
  (params (OverlappedComponent :type Primitive%20Component%20Object%20Reference) (OtherActor :type Actor%20Object%20Reference) (OtherComp :type Primitive%20Component%20Object%20Reference) (OtherBodyIndex :type Integer) (bFromSweep :type Boolean) (SweepResult :type Hit%20Result%20Structure%20%28by%20ref%29))
  ;[1 1 1] On overlap with charachter, start damage tick
  (if (not (Utilities|Time|IsValidTimerHandle (Variables|RebelX|DamageVolume|GetDamage%20Tick%20Timer)))
    (Utilities|Casting|CastToCharacter OtherActor)
    (bind _returnvalue (Utilities|Time|SetTimerbyEvent (delegate Custom|Event%20Damage%20Tick) (Variables|RebelX|DamageVolume|GetDamage%20Tick%20Duration) true))
    (Variables|RebelX|DamageVolume|SetDamage%20Tick%20Timer _returnvalue)))

(event OnComponentEndOverlap(Box)
  (params (OverlappedComponent :type Primitive%20Component%20Object%20Reference) (OtherActor :type Actor%20Object%20Reference) (OtherComp :type Primitive%20Component%20Object%20Reference) (OtherBodyIndex :type Integer))
  ;[1 1 1] Stop timer if no overlapps with charachter.
  (if (not (Utilities|Array|IsValidIndex (Collision|GetOverlappingActors "/Script/Engine.Character" :!class /Script/Engine.Actor)))
    (Utilities|Time|ClearandInvalidateTimerbyHandle (Variables|RebelX|DamageVolume|GetDamage%20Tick%20Timer))))

(event Custom|Event%20Damage%20Tick
  ;[1 1 1] Damge tick, applies damage to overlapped charachters.
  (for _array_element (Collision|GetOverlappingActors "/Script/Engine.Character" :!class /Script/Engine.Actor)
    (Game|Damage|ApplyDamage _array_element (Variables|RebelX|DamageVolume|GetDamage%20Per%20Tick) 0 self)))

(event Custom|OpenPuzzleDoor
  (Variables|Default|SetStartLocation (Transformation|GetActorLocation))
  (bind _alpha (Timeline|Timeline PlayFromStart)
    (:Update
      (Transformation|SetActorLocation (Math|Vector|Lerp(Vector) (Variables|Default|GetStartLocation) (- (Variables|Default|GetStartLocation) "0.000000,0.000000,400.000000") _alpha) false false)
      (Development|PrintString "000"))))

(event EventUnlock
  (params (Locks :type Integer))
  (bind _output_get (Variables|Default|SetCurrentLocks (+ (Variables|Default|GetCurrentLocks) Locks)))
  (if (== _output_get (Variables|Default|GetLocksRequired))
    (Utilities|FlowControl|DoOnce false
      (:Completed
        (CallFunction|OpenPuzzleDoor)
        (bind _returnvalue (Sequencer|Player|CreateLevelSequencePlayer "/Game/L3/LevelSequence/LS_03.LS_03"))
        (Sequencer|Player|Play _returnvalue :!class /Script/MovieScene.MovieSceneSequencePlayer)))))

(event Input|KeyboardEvents|E
  (params (Key :type Key%20Structure :default "None")))

(fn ConstructionScript)