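; BP_DialogueTrigger is a box trigger that plays a line of dialogue once when the Player_RebelX character enters it.
; BeginPlay caches the player reference after a short delay.
; The first matching overlap passes the trigger's DialogueID to the player, adds a WBP_Dialogue widget to the viewport and calls PlayDialogue on the player.
; The widget is removed after a fixed five-second delay.
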(event OnComponentBeginOverlap(Box)
  (params (OverlappedComponent :type Primitive%20Component%20Object%20Reference) (OtherActor :type Actor%20Object%20Reference) (OtherComp :type Primitive%20Component%20Object%20Reference) (OtherBodyIndex :type Integer) (bFromSweep :type Boolean) (SweepResult :type Hit%20Result%20Structure%20%28by%20ref%29))
  (if (== OtherActor (Variables|Default|GetAs%20Player%20Rebel%20X))
    (Utilities|FlowControl|DoOnce false
      (:Completed
        (Variables|/Game/RebelX_Core/Blueprints/Player_RebelX.Player_RebelX_C|SetDialogueID (Variables|Default|GetAs%20Player%20Rebel%20X) (Variables|Default|GetDialogue%20ID))
        (bind _returnvalue (UserInterface|CreateWidget "/Game/Widget/WBP_Dialogue.WBP_Dialogue_C"))
        (Variables|Default|SetNewVar _returnvalue)
        (UserInterface|Viewport|AddtoViewport _returnvalue 0)
        (Default|PlayDialogue (Variables|Default|GetAs%20Player%20Rebel%20X))
        (Utilities|FlowControl|Delay 5.0)
        (Widget|RemovefromParent (Variables|Default|GetNewVar))))))

(event Custom|11)

(event EventBeginPlay
  (Utilities|FlowControl|Delay 0.5)
  (bind _asplayer_rebel_x (Utilities|Casting|CastToPlayer_RebelX (Game|GetPlayerCharacter 0)))
  (Variables|Default|SetAs%20Player%20Rebel%20X _asplayer_rebel_x))

(event Collision|EventActorBeginOverlap
  (params (OtherActor :type Actor%20Object%20Reference)))

(event EventTick
  (params (DeltaSeconds :type Float%20%28single-precision%29)))

(fn ConstructionScript)