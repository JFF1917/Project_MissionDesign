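; Rotating puzzle piece that feeds unlock progress to two referenced doors.
; Construction gives the box a random 90, 180 or 270 degree yaw and applies the unlock material.
; While Player_RebelX overlaps the interact volume, a widget shows and E rotates the box a quarter turn via timeline, blocked mid-rotation.
; Box1 overlapping Box2 sends +1 to both doors' Unlock, and -1 when the overlap ends.
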(event OnComponentBeginOverlap(BoxInteract)
  (params (OverlappedComponent :type Primitive%20Component%20Object%20Reference) (OtherActor :type Actor%20Object%20Reference) (OtherComp :type Primitive%20Component%20Object%20Reference) (OtherBodyIndex :type Integer) (bFromSweep :type Boolean) (SweepResult :type Hit%20Result%20Structure%20%28by%20ref%29))
  (Utilities|Casting|CastToPlayer_RebelX OtherActor)
  (Input|EnableInput (Game|GetPlayerController 0))
  (Rendering|SetVisibility (Variables|Default|GetWidget) true false))

(event OnComponentEndOverlap(BoxInteract)
  (params (OverlappedComponent :type Primitive%20Component%20Object%20Reference) (OtherActor :type Actor%20Object%20Reference) (OtherComp :type Primitive%20Component%20Object%20Reference) (OtherBodyIndex :type Integer))
  (Utilities|Casting|CastToPlayer_RebelX OtherActor)
  (Input|DisableInput (Game|GetPlayerController 0))
  (Rendering|SetVisibility (Variables|Default|GetWidget) false false))

(event OnComponentBeginOverlap(Box1)
  (params (OverlappedComponent :type Primitive%20Component%20Object%20Reference) (OtherActor :type Actor%20Object%20Reference) (OtherComp :type Primitive%20Component%20Object%20Reference) (OtherBodyIndex :type Integer) (bFromSweep :type Boolean) (SweepResult :type Hit%20Result%20Structure%20%28by%20ref%29))
  (if (== OtherComp (Variables|Default|GetBox2))
    (Utilities|FlowControl|Sequence
      (:then_0
        (Default|Unlock (Variables|Default|GetDoorRef) 1))
      (:then_1
        (Default|Unlock (Variables|Default|GetDoorRef2) 1)))))

(event OnComponentEndOverlap(Box1)
  (params (OverlappedComponent :type Primitive%20Component%20Object%20Reference) (OtherActor :type Actor%20Object%20Reference) (OtherComp :type Primitive%20Component%20Object%20Reference) (OtherBodyIndex :type Integer))
  (if (== OtherComp (Variables|Default|GetBox2))
    (Utilities|FlowControl|Sequence
      (:then_0
        (Default|Unlock (Variables|Default|GetDoorRef) -1))
      (:then_1
        (Default|Unlock (Variables|Default|GetDoorRef2) -1)))))

(event Input|KeyboardEvents|E
  (params (Key :type Key%20Structure :default "None"))
  (:Pressed
    (if (Variables|Default|GetCanRotate)
      (Variables|Default|SetCanRotate false)
      (Variables|Default|SetStartRotation (Variables|/Script/Engine.SceneComponent|GetRelativeRotation (Variables|Default|GetBox)))
      (bind _alpha (Timeline|Rotation PlayFromStart)
        (:Update
          (Transformation|SetRelativeRotation (Variables|Default|GetBox) (Math|Rotator|Lerp(Rotator) (Variables|Default|GetStartRotation) (Math|Rotator|MakeRotator 0.0 0.0 (+ (.Yaw (Math|Rotator|BreakRotator (Variables|Default|GetStartRotation))) 9e+01)) _alpha) false false))
        (:Finished
          (Variables|Default|SetCanRotate true))))))

(fn ConstructionScript
  (bind _unlockmat (Variables|Default|GetUnlockMat))
  (Transformation|SetRelativeRotation (Variables|Default|GetBox) (Math|Rotator|MakeRotator 0.0 0.0 (Utilities|Select :Index (Math|Random|RandomIntegerinRange 0 2) :Option%200 9e+01 :Option%201 1.8e+02 :Option%202 2.7e+02)) false false)
  (Rendering|Material|SetMaterial (Variables|Default|GetBox) 2 _unlockmat)
  (Rendering|Material|SetMaterial (Variables|Default|GetPlane) 0 _unlockmat))

(fn GetAmmoInfo
  (return false "NewEnumerator0"))

(fn GetCrosshairPrompt
  (return "" ""))

(fn GetHealthInfo
  (return false 0.0))

(fn GetInteractionType
  (return false "NewEnumerator4"))

(fn GetIsConsumeable
  (return false))

(fn GetSceneInfo
  (return false))