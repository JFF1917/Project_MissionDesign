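; BP_NormalDoor1 is a proximity door that slides open when the player presses E.
; Player_RebelX entering the Box trigger enables input and shows a prompt widget; leaving reverses both.
; The debug E key plays a timeline that moves the Cube and sets the Box to a fixed relative position.
; OpenDoor is an empty event, and the numpad glass widget toggle is disconnected.
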(event OnComponentBeginOverlap(Box)
  (params (OverlappedComponent :type Primitive%20Component%20Object%20Reference) (OtherActor :type Actor%20Object%20Reference) (OtherComp :type Primitive%20Component%20Object%20Reference) (OtherBodyIndex :type Integer) (bFromSweep :type Boolean) (SweepResult :type Hit%20Result%20Structure%20%28by%20ref%29))
  (Utilities|Casting|CastToPlayer_RebelX OtherActor)
  (Input|EnableInput (Game|GetPlayerController 0))
  (Rendering|SetVisibility (Variables|Default|GetWidget) true false))

(event OnComponentEndOverlap(Box)
  (params (OverlappedComponent :type Primitive%20Component%20Object%20Reference) (OtherActor :type Actor%20Object%20Reference) (OtherComp :type Primitive%20Component%20Object%20Reference) (OtherBodyIndex :type Integer))
  (Utilities|Casting|CastToPlayer_RebelX OtherActor)
  (Input|DisableInput (Game|GetPlayerController 0))
  (Rendering|SetVisibility (Variables|Default|GetWidget) false false))

(event Custom|OpenDoor)

(event EventBeginPlay)

(event Collision|EventActorBeginOverlap
  (params (OtherActor :type Actor%20Object%20Reference)))

(event EventTick
  (params (DeltaSeconds :type Float%20%28single-precision%29)))

(event Input|KeyboardEvents|DebugKeyE
  (params (Key :type Key%20Structure) (ActionValue :type Input%20Action%20Value%20Structure))
  (:Pressed
    (bind _newtrack_0 (Timeline|TimeLine Play)
      (:Update
        (Transformation|SetRelativeLocation (Variables|Default|GetCube) _newtrack_0 false false)
        (Transformation|SetRelativeLocation (Variables|Default|GetBox) "0.000000,0.000000,200.000000" false false)))))

(fn ConstructionScript)