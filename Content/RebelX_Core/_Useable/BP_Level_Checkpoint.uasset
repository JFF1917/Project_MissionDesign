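; BP_Level_Checkpoint is a one-shot checkpoint trigger volume that updates the player's respawn point.
; When a Player_RebelX overlaps its box, it saves that player's current transform as RespawnTransform and posts NotificationText to the attached HUD.
; It then destroys itself after a short delay.
; The construction script sizes the trigger box from the BoxExtent variable.
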(event OnComponentBeginOverlap(Box)
  (params (OverlappedComponent :type Primitive%20Component%20Object%20Reference) (OtherActor :type Actor%20Object%20Reference) (OtherComp :type Primitive%20Component%20Object%20Reference) (OtherBodyIndex :type Integer) (bFromSweep :type Boolean) (SweepResult :type Hit%20Result%20Structure%20%28by%20ref%29))
  (bind _asplayer_rebel_x (Utilities|Casting|CastToPlayer_RebelX OtherActor))
  (Variables|/Game/RebelX_Core/Blueprints/Player_RebelX.Player_RebelX_C|SetRespawn%20Transform _asplayer_rebel_x (Transformation|GetActorTransform _asplayer_rebel_x))
  (Class|BPIHUD|AddNotificaiton(Message) (Default|GetAttachedHUD _asplayer_rebel_x) (Variables|RebelX|Checkpoint|GetNotification%20Text))
  (Utilities|FlowControl|Delay 0.2)
  (Actor|DestroyActor))

(event EventBeginPlay)

(event Collision|EventActorBeginOverlap
  (params (OtherActor :type Actor%20Object%20Reference)))

(event EventTick
  (params (DeltaSeconds :type Float%20%28single-precision%29)))

(fn ConstructionScript
  (Components|Box|SetBoxExtent (Variables|Default|GetBox) (Variables|RebelX|Checkpoint|GetBox%20Extent) true))