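; BP_Scene_Button1 is an interactable scene button that broadcasts a ButtonPressed event when activated, optionally gated by a keycard.
; When a key is required, it checks the player's backpack for its KeyID; failure plays a Type-based elevator dialogue and flashes the light red.
; A successful press turns the light green through a DoOnce, which resets after a short delay if Retriggerable.
; Interaction interface functions supply the crosshair prompt and mark it non-consumable.
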(event EventActivateSceneObject
  (if (Variables|Default|GetNeedKey?)
    (bind _asplayer_rebel_x (Utilities|Casting|CastToPlayer_RebelX (Game|GetPlayerCharacter 0)))
    (bind _asbp_backpack (Utilities|Casting|CastToBP_Backpack (Variables|/Game/RebelX_Core/Blueprints/Player_RebelX.Player_RebelX_C|GetVariable_Backpack _asplayer_rebel_x)))
    (if (Utilities|Array|Get(acopy) (Variables|/Game/RX_C_Bailey_Content/Blueprints/BP_Backpack.BP_Backpack_C|GetKeycard%20IDs _asbp_backpack) (Variables|Default|GetKeyID))
      (Utilities|FlowControl|DoOnce false :!label _label
        (:Completed
          (Default|CallButtonPressed)
          (Rendering|Components|Light|SetLightColor (Variables|Default|GetPointLight) "(R=0.000000,G=1.000000,B=0.000000,A=1.000000)" true)
          (if (Variables|Default|GetbRetriggerable)
            (Utilities|FlowControl|Delay 0.5)
            (Rendering|Components|Light|SetLightColor (Variables|Default|GetPointLight) "(R=1.000000,G=1.000000,B=1.000000,A=1.000000)" true)
            (goto _label Reset))))
      (else
        (Utilities|FlowControl|Sequence
          (:then_0
            (switch string (Variables|Default|GetType)
              (:Elevator
                (Variables|Default|SetDialogue%20ID "Dialogue_70"))
              (:ElevatorVIP
                (Variables|Default|SetDialogue%20ID "Dialogue_71")))
            (Variables|/Game/RebelX_Core/Blueprints/Player_RebelX.Player_RebelX_C|SetDialogueID _asplayer_rebel_x (Variables|Default|GetDialogue%20ID))
            (UserInterface|Viewport|AddtoViewport (Variables|/Game/RebelX_Core/Blueprints/Player_RebelX.Player_RebelX_C|GetWBP_Dialogue_Ins _asplayer_rebel_x) 0)
            (Default|PlayDialogue _asplayer_rebel_x))
          (:then_1
            (Rendering|Components|Light|SetLightColor (Variables|Default|GetPointLight) "(R=1.000000,G=0.000000,B=0.003374,A=1.000000)" true)
            (Utilities|FlowControl|Delay 0.5)
            (Rendering|Components|Light|SetLightColor (Variables|Default|GetPointLight) "(R=1.000000,G=1.000000,B=1.000000,A=1.000000)" true)))))
    (else
      (goto _label))))

(fn ConstructionScript)

(fn GetInteractionType
  (return true "NewEnumerator2"))

(fn GetIsConsumeable
  (return false))

(fn GetCrosshairPrompt
  (return (Variables|Default|GetInteraction%20Message) "[E] INTERACT"))