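; X13 pistol weapon Blueprint that extends its LPAMG parent with forestock, barrel, rail and front ironsight parts, including skins and icons.
; A randomized forestock selects the matching barrel and icons by array index, while the grip selects fire rate multiplier and first-person fire montage.
; Grip, laser and scope sockets move to the rail, which hides when empty; muzzles move to the barrel.
; Aim offset compensates for the rail's scope socket position.
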(event EventLPAMG-onSetAttachmentsScale
  (params (Scale :type Float%20%28double-precision%29))
  (|CallParentFunction Scale)
  (Transformation|SetRelativeScale3D (Variables|Default|GetSocket%20Rail) (Math|Conversions|ToVector(Float) Scale)))

(fn ConstructionScript
  (|CallParentFunction))

(fn LPAMG-GetRateOfFire
  (return (* (Variables|Default|GetRate%20Of%20Fire) (Utilities|Array|Get(acopy) (Variables|InfimaGames|Weapon|Settings|GetArray%20Fire%20Rate%20Multipliers) (select (CallFunction|AreAttachmentsVisiblePure) (Utilities|Array|FindItem (Variables|Default|GetArray%20Static%20Mesh%20Grips) (Variables|/Script/Engine.StaticMeshComponent|GetStaticMesh (Variables|Default|GetMesh%20Grip))) 0)))))

(fn LPAMG-GetFirstPersonMontageCharacterFire
  (return (Utilities|Array|Get(acopy) (Variables|InfimaGames|Weapon|Animations|FirstPerson|GetArray%20Fire%20Montages) (select (CallFunction|AreAttachmentsVisiblePure) (Utilities|Array|FindItem (Variables|Default|GetArray%20Static%20Mesh%20Grips) (Variables|/Script/Engine.StaticMeshComponent|GetStaticMesh (Variables|Default|GetMesh%20Grip))) 0))))

(fn RandomizeSkin
  (|CallParentFunction)
  (Default|Applyto (Variables|Default|GetSkin%20Equipped) (Variables|Default|GetMesh%20Forestock) "Forestock") ; Forestock
  (Default|Applyto (Variables|Default|GetSkin%20Equipped) (Variables|Default|GetMesh%20Barrel) "Barrel") ; Barrel
  (Default|Applyto (Variables|Default|GetSkin%20Equipped) (Variables|Default|GetMesh%20Rail) "Rail") ; Rail
  (Default|Applyto (Variables|Default|GetSkin%20Equipped) (Variables|Default|GetMesh%20Ironsight%20Front) "Ironsights") ; Ironsights
)

(fn LPAMG-GetExtraAimOffset
  (return (Math|Vector|NegateVector (- (.Location (Math|Transform|BreakTransform (Transformation|GetSocketTransform (Variables|Default|GetMesh%20Rail) "SOCKET_Scope" "RTS_Actor"))) (.Location (Math|Transform|BreakTransform (Transformation|GetSocketTransform (Variables|Default|GetWeapon) "SOCKET_Scope" "RTS_Actor")))))))

(fn LPAMG-GetTextureIconMuzzle
  (return (select (== (Utilities|Array|FindItem (Variables|Default|GetArray%20Static%20Mesh%20Muzzles) (Variables|/Script/Engine.StaticMeshComponent|GetStaticMesh (Variables|Default|GetMesh%20Muzzle))) 0) 0 (select (CallFunction|AreAttachmentsVisiblePure) (Utilities|Array|Get(acopy) (Variables|InfimaGames|Weapon|Icons|GetArray%20Texture%20Icon%20Muzzles%20Extended) (Utilities|Array|FindItem (Variables|InfimaGames|Weapon|Attachments|GetArray%20Static%20Mesh%20Forestocks) (Variables|/Script/Engine.StaticMeshComponent|GetStaticMesh (Variables|Default|GetMesh%20Forestock)))) 0))))

(fn LPAMG-GetTextureIconForestock
  (return (Utilities|Array|Get(acopy) (Variables|InfimaGames|Weapon|Icons|GetArray%20Texture%20Icon%20Forestocks) (Utilities|Array|FindItem (Variables|InfimaGames|Weapon|Attachments|GetArray%20Static%20Mesh%20Forestocks) (Variables|/Script/Engine.StaticMeshComponent|GetStaticMesh (Variables|Default|GetMesh%20Forestock))))))

(fn AreRailsInvisible
  (return (and (and (not (Utilities|IsValid (Variables|/Script/Engine.StaticMeshComponent|GetStaticMesh (Variables|Default|GetMesh%20Laser)))) (not (Utilities|IsValid (Variables|/Script/Engine.StaticMeshComponent|GetStaticMesh (Variables|Default|GetMesh%20Scope))))) (not (Utilities|IsValid (Variables|/Script/Engine.StaticMeshComponent|GetStaticMesh (Variables|Default|GetMesh%20Grip)))))))

(fn LPAMG-GetTextureIconRails
  (return (select (or (InfimaGames|Weapon|AreRailsInvisible) (not (CallFunction|AreAttachmentsVisiblePure))) 0 (Variables|InfimaGames|Weapon|Icons|GetArray%20Texture%20Icon%20Rails))))

(fn GetSocketGripParent
  (return (Variables|Default|GetMesh%20Rail) (.Socket%20Name (|CallParentFunction))))

(fn GetSocketMuzzleParent
  (return (Variables|Default|GetMesh%20Barrel) (.Socket%20Name (|CallParentFunction))))

(fn GetSocketLaserParent
  (return (Variables|Default|GetMesh%20Rail) (.Socket%20Name (|CallParentFunction))))

(fn GetSocketScopeParent
  (return (Variables|Default|GetMesh%20Rail) (.Socket%20Name (|CallParentFunction))))

(fn GetSocketIronsightsParent
  (return (.Parent (|CallParentFunction)) "SOCKET_Ironsights"))

(fn LPAMG-GetTextureIconIronsightsFront
  (return (Utilities|Array|Get(acopy) (Variables|Default|GetArray%20Texture%20Icon%20Ironsights%20Front) (Utilities|Array|FindItem (Variables|InfimaGames|Weapon|Attachments|GetArray%20Static%20Mesh%20Forestocks) (Variables|/Script/Engine.StaticMeshComponent|GetStaticMesh (Variables|Default|GetMesh%20Forestock))))))

(fn RandomizeAttachmentMeshes
  (|CallParentFunction)
  (Components|StaticMesh|SetStaticMesh (Variables|Default|GetMesh%20Forestock) (.OutItem (Utilities|Array|RandomFromStream (Variables|InfimaGames|Weapon|Attachments|GetArray%20Static%20Mesh%20Forestocks) (Variables|Default|GetRandom%20Stream))) :!pinned true) ; Forestock
  (Components|StaticMesh|SetStaticMesh (Variables|Default|GetMesh%20Barrel) (Utilities|Array|Get(acopy) (Variables|InfimaGames|Weapon|Attachments|GetArray%20Static%20Mesh%20Barrels) (Utilities|Array|FindItem (Variables|InfimaGames|Weapon|Attachments|GetArray%20Static%20Mesh%20Forestocks) (Variables|/Script/Engine.StaticMeshComponent|GetStaticMesh (Variables|Default|GetMesh%20Forestock)))) :!pinned true) ; Barrels
  (Development|SetHiddeninGame (Variables|Default|GetMesh%20Rail) (InfimaGames|Weapon|AreRailsInvisible) false) ; This node makes sure to hide the rail\non the handgun when there's no attachments\nthat would be placed on it.\n\nThis is kind of cool so we can show it without\nit too.
)

(fn GetCrosshairPrompt
  (return "X13 - PISTOL" "[E] PICKUP"))