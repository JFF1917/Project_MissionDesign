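; BP_LPAMG_Casing is a weapon shell casing actor that flies, tumbles and removes itself after a short time.
; The Apply Impulse interface event sets the ProjectileMovement velocity from a direction and strength.
; Tick spins the mesh on pitch and yaw, re-rolling a random speed each frame.
; BeginPlay waits a random lifetime, plays a 2D sound at varied volume, then destroys the actor.
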(event EventTick
  (params (DeltaSeconds :type Float%20%28single-precision%29))
  (bind _minrotationspeed (Variables|InfimaGames|Casing|GetMinRotationSpeed))
  (bind _maxrotationspeed (Variables|InfimaGames|Casing|GetMaxRotationSpeed))
  (bind _returnvalue (Math|Random|RandomFloatinRange _minrotationspeed _maxrotationspeed))
  (bind _returnvalue_2 (* DeltaSeconds _returnvalue))
  (Transformation|AddRelativeRotation (Variables|Default|GetMesh) (Math|Rotator|MakeRotator 0.0 _returnvalue_2 _returnvalue_2) false false))

(event EventBeginPlay
  (bind _casing_destroy_time (Variables|InfimaGames|Casing|GetCasing%20Destroy%20Time))
  (bind (_x _y) (Math|Vector2D|BreakVector2D _casing_destroy_time))
  (|CallParentFunction)
  (Utilities|FlowControl|Delay (Math|Random|RandomFloatinRange _x _y))
  (Audio|PlaySound2D (Variables|InfimaGames|Casing|GetSound) (Math|Random|RandomFloatinRange 0.8 1.2) 1.0 0.0 0 0 false)
  (Actor|DestroyActor))

(event EventLPAMG-ApplyImpulse
  (params (Direction :type Vector :default "0, 0, 0") (Strength :type Vector :default "0, 0, 0"))
  ;[0.875 0 1 1 12] Apply Impulse
  (Variables|/Script/Engine.MovementComponent|SetVelocity (Variables|Default|GetProjectile%20Movement) (* Direction Strength)))

(fn ConstructionScript)