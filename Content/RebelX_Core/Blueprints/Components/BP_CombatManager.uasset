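; Combat manager component that tracks enemies in combat, starts and ends the combat state, and drives combat music and chimes.
; Added enemies target the player and randomly claim a control point with free capacity, taking a different stance if none is found.
; Starting combat also pulls in active enemies from attached encounter managers.
; A shared attack token pool grants or refuses requests, and a tick-driven debug printout shows the state.
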(event Custom|End%20Combat%20Music
  (bind _combatmusic (Variables|Default|GetCombatMusic))
  ;[1 1 1] Music
  (Utilities|FlowControl|Delay 1.0)
  (Utilities|FlowControl|Sequence
    (:then_0
      (if (Variables|RebelX|CombatManager|Audio|GetCombat%20Chimes)
        (Audio|PlaySound2D "/Game/RebelX_Core/Audio/FX/SC_FX_CombatEnded.SC_FX_CombatEnded" 2.0 1.0 0.0 0 0)))
    (:then_1
      (Utilities|IsValid _combatmusic
        (:Is%20Valid
          (Audio|Components|Audio|Stop _combatmusic)
          (Components|DestroyComponent _combatmusic))))))

(event Custom|Start%20Combat%20Music
  (Utilities|FlowControl|Sequence
    (:then_0
      (if (Variables|RebelX|CombatManager|Audio|GetCombat%20Chimes)
        ;[1 1 0] Need music system
        (Audio|PlaySound2D "/Game/RebelX_Core/Audio/FX/SC_FX_CombatStarted.SC_FX_CombatStarted" 2.0 1.0 0.0 0 0)
        (Audio|PlaySound2D "/Game/RebelX_Core/Audio/FX/W_FX_CombatStarted.W_FX_CombatStarted" 0.5 1.0 0.0 0 0)))
    (:then_1
      ;[1 1 0] Combat Music
      (if (Variables|RebelX|CombatManager|Audio|GetCombat%20Music)
        (Utilities|IsValid (Variables|Default|GetCombatMusic)
          (:Is%20Not%20Valid
            (bind _returnvalue (Audio|SpawnSoundAttached "/Game/RebelX_Core/Audio/FX/W_CombatMusic.W_CombatMusic" (Variables|/Script/Engine.Actor|GetRootComponent (Game|Player|GetPlayerPawn 0)) "None" "0, 0, 0" "0, 0, 0" "KeepRelativeOffset" false 1.0 1.0 0.0 0 0))
            (bind _output_get (Variables|Default|SetCombatMusic _returnvalue))
            (Class|AudioComponent|SetUISound _output_get true)))))))

(event EventRemoveContolPoints
  (params (Control%20Points :type Array%20of%20Actor%20Object%20References))
  ;[1 1 1] Remove Control Points
  (for _array_element Control%20Points
    (Utilities|Map|Remove (Variables|RebelX|CombatManager|Encounters|GetControl%20Points) _array_element)))

(event EventAttachControlPoints
  (params (Control%20Points :type Map%20of%20Actor%20Object%20References%20to%20Integers))
  ;[1 1 1] Attach Control Points
  (bind _keys (Utilities|Map|Keys Control%20Points))
  (for _array_element _keys
    (Utilities|Map|Add (Variables|RebelX|CombatManager|Encounters|GetControl%20Points) _array_element (.Value (Utilities|Map|Find Control%20Points _array_element)))))

(event EventAddtoCombat
  (params (Actor :type Actor%20Object%20Reference))
  (bind _returnvalue (AI|GetAIController Actor))
  (bind _control_points (Variables|RebelX|CombatManager|Encounters|GetControl%20Points))
  ;[1 1 1] Add to Combat
  (Utilities|FlowControl|DelayUntilNextTick)
  (Utilities|FlowControl|Sequence
    (:then_0
      (if (not (Utilities|Map|Contains (Variables|RebelX|CombatManager|Encounters|GetEnemy%20Characters) Actor))
        (|GraphAddToCombat Actor)
        (bind (_return_value _control_point) (CallFunction|RequestControlPoint Actor))
        (if _return_value
          (Class|BPIAIController|SetEnemyStance(Message) _returnvalue "NewEnumerator3")
          (Class|BPIAIController|SetControlPoint(Message) _returnvalue _control_point)
          (Utilities|Map|Add (Variables|RebelX|CombatManager|Encounters|GetEnemy%20Characters) Actor "NewEnumerator3")
          (Utilities|Map|Add (Variables|RebelX|CombatManager|Encounters|GetEnemy%20Control%20Point%20Assignments) Actor _control_point)
          (Utilities|Map|Add _control_points _control_point (+ (.Value (Utilities|Map|Find _control_points _control_point)) -1))
          (else
            (Class|BPIAIController|SetEnemyStance(Message) (AI|GetAIController Actor) "NewEnumerator2")
            (Utilities|Map|Add (Variables|RebelX|CombatManager|Encounters|GetEnemy%20Characters) Actor "NewEnumerator2")))))
    (:then_1
      (if (not (Variables|RebelX|CombatManager|GetCombat%20Active))
        (CallFunction|StartCombat)
        (CallFunction|AlertEnemeisfromAttachedEncounter Actor)))))

(event EventRemoveEncounterManager
  (params (Encounter%20Manager :type Actor%20Object%20Reference))
  ;[1 1 1] Remove Encounter
  (Utilities|Set|Remove (Variables|RebelX|CombatManager|Encounters|GetCurrent%20Encounters) Encounter%20Manager))

(event EventRemovefromCombat
  (params (Actor :type Actor%20Object%20Reference))
  (bind _control_points (Variables|RebelX|CombatManager|Encounters|GetControl%20Points))
  (bind _enemy_control_point_assignments (Variables|RebelX|CombatManager|Encounters|GetEnemy%20Control%20Point%20Assignments))
  (bind _value (Utilities|Map|Find _enemy_control_point_assignments Actor))
  (Utilities|Map|Remove (Variables|RebelX|CombatManager|Encounters|GetEnemy%20Characters) Actor)
  (CallFunction|DebugLog (Utilities|String|Append "Removing enemy from combat: " (Utilities|GetDisplayName Actor)) "NewEnumerator0" "None" (Variables|RebelX|GetDebug))
  (Utilities|IsValid _value
    (:Is%20Valid
      (Utilities|Map|Add _control_points _value (+ (.Value (Utilities|Map|Find _control_points _value)) 1))
      (Utilities|Map|Remove (Variables|RebelX|CombatManager|Encounters|GetEnemy%20Control%20Point%20Assignments) Actor))))

(event EventAttachEncounterManager
  (params (Encounter%20Manager :type Actor%20Object%20Reference))
  ;[1 1 1] Attach Encounter
  (Utilities|Set|Add (Variables|RebelX|CombatManager|Encounters|GetCurrent%20Encounters) Encounter%20Manager)
  (if (Variables|RebelX|CombatManager|GetCombat%20Active)
    (CallFunction|AlertEnemeisfromAttachedEncounter)))

(event EventBeginPlay
  (if (Variables|RebelX|GetDebugInfo)
    (Components|Tick|SetComponentTickEnabled true)))

(event EventTick
  (params (DeltaSeconds :type Float%20%28single-precision%29))
  (CallFunction|PrintDebugInfo))

(event EventResetAttackTokens
  (params (Attack%20Tokens :type Integer))
  ;[1 1 1] Reset Attack Tokens
  (Variables|RebelX|CombatManager|SetAvalible%20Attack%20Tokens Attack%20Tokens))

(fn SendtoAttack
  (params (Charachter :type Character%20Object%20Reference))
  (AI|Components|Blackboard|SetValueasEnum (AI|GetBlackboard (AI|GetAIController Charachter)) (Utilities|Name|MakeLiteralName "Stance") (Utilities|Enum|LiteralenumE_EnemyStances "NewEnumerator1")))

(fn UpdateCombatMusicConfig
  (params (bPlayCombatMusic :type Boolean) (bPlayCombatChimes :type Boolean))
  (Variables|RebelX|CombatManager|Audio|SetCombat%20Music bPlayCombatMusic)
  (Variables|RebelX|CombatManager|Audio|SetCombat%20Chimes bPlayCombatChimes))

(fn AlertEnemeisfromAttachedEncounter
  (params (Alerter :type Actor%20Object%20Reference))
  (bind _result (Utilities|Set|ToArray (Variables|RebelX|CombatManager|Encounters|GetCurrent%20Encounters)))
  (for _array_element _result
    (bind _enemies (Class|BPIEncounterManager|GetActiveEnemies(Message) _array_element))
    (Utilities|Array|RemoveItem _enemies Alerter)
    (for _array_element_2 _enemies
      (CallFunction|AddtoCombat _array_element_2))))

(fn StartCombat
  (CallFunction|DebugLog "Starting Combat..." "NewEnumerator0" "Combat" (Variables|RebelX|GetDebug))
  (Variables|RebelX|CombatManager|SetCombat%20Active true)
  (Default|CallCombatStarted)
  (CallFunction|StartCombatMusic))

(fn EndCombat
  (CallFunction|DebugLog "Ending Combat..." "NewEnumerator0" "Combat" (Variables|RebelX|GetDebug))
  (Variables|RebelX|CombatManager|SetCombat%20Active false)
  (Default|CallCombatEnded)
  (CallFunction|EndCombatMusic))

(fn PrintDebugInfo
  (Utilities|FlowControl|Sequence
    (:then_0
      (Development|PrintString "COMBAT MANAGER DEBUG" true true "(R=1.000000,G=0.000000,B=0.027671,A=1.000000)" 2.0 "Debug Header"))
    (:then_1
      (Development|PrintString (Utilities|String|Append "AVALIBLE ATTACK TOKENS = " (Utilities|String|ToString(Integer) (Variables|RebelX|CombatManager|GetAvalible%20Attack%20Tokens))) true true "(R=1.000000,G=1.000000,B=1.000000,A=1.000000)" 2.0 "Tokens"))
    (:then_2
      (Development|PrintString "ATTACTHED ENEMIES 
--------------------- " true true "(R=1.000000,G=1.000000,B=1.000000,A=1.000000)" 2.0 "Enemeis Header")
      (bind _keys (Utilities|Map|Keys (Variables|RebelX|CombatManager|Encounters|GetEnemy%20Characters)))
      (for _array_element _keys
        (LocalVariables|SetEnemies (Utilities|String|Append (Utilities|GetDisplayName _array_element) " 
" (LocalVariables|GetEnemies))))
      (Development|PrintString (LocalVariables|GetEnemies) true true "(R=1.000000,G=1.000000,B=1.000000,A=1.000000)" 2.0 "Enemies"))
    (:then_3
      (Development|PrintString "ATTATCHED ENCOUNTERS 
-------------------------- " true true "(R=1.000000,G=1.000000,B=1.000000,A=1.000000)" 2.0 "Encounter Header")
      (bind _result (Utilities|Set|ToArray (Variables|RebelX|CombatManager|Encounters|GetCurrent%20Encounters)))
      (for _array_element_2 _result
        (LocalVariables|SetEncounters (Utilities|String|Append (Utilities|GetDisplayName _array_element_2) " 
" (LocalVariables|GetEncounters))))
      (Development|PrintString (LocalVariables|GetEncounters) true true "(R=1.000000,G=1.000000,B=1.000000,A=1.000000)" 2.0 "Encounters"))
    (:then_4
      (Development|PrintString "ATTATCHED CONTROL POINTS 
------------------------------" true true "(R=1.000000,G=1.000000,B=1.000000,A=1.000000)" 2.0 "Control Point Header")
      (bind _keys_2 (Utilities|Map|Keys (Variables|RebelX|CombatManager|Encounters|GetControl%20Points)))
      (for _array_element_3 _keys_2
        (LocalVariables|SetControl%20Points (Utilities|String|Append (Utilities|GetDisplayName _array_element_3) " 
" (LocalVariables|GetControl%20Points))))
      (Development|PrintString (LocalVariables|GetControl%20Points) true true "(R=1.000000,G=1.000000,B=1.000000,A=1.000000)" 2.0 "Control Points"))))

(fn GetEnemyControlPointAsignments
  (return (Variables|RebelX|CombatManager|Encounters|GetEnemy%20Control%20Point%20Assignments)))

(fn InCombat
  (return (Variables|RebelX|CombatManager|GetCombat%20Active)))

(fn RequestAttackTokens
  (params (Requested%20Attack%20Tokens :type Integer))
  (if (<= Requested%20Attack%20Tokens (Variables|RebelX|CombatManager|GetAvalible%20Attack%20Tokens))
    (bind _output_get (Variables|RebelX|CombatManager|SetAvalible%20Attack%20Tokens (- (Variables|RebelX|CombatManager|GetAvalible%20Attack%20Tokens) Requested%20Attack%20Tokens)))
    (CallFunction|DebugLog (Utilities|String|Append "Attack Tokens: " (Utilities|String|ToString(Integer) _output_get)) "NewEnumerator0" "Attack Tokens" (Variables|RebelX|GetDebug))
    (return true Requested%20Attack%20Tokens)
    (else
      (return false 0))))

(fn RequestControlPoint
  (params (Actor :type Actor%20Object%20Reference))
  (bind _enemy_control_point_assignments (Variables|RebelX|CombatManager|Encounters|GetEnemy%20Control%20Point%20Assignments))
  (bind (_value _returnvalue) (Utilities|Map|Find _enemy_control_point_assignments Actor))
  (bind _keys (Utilities|Map|Keys (Variables|RebelX|CombatManager|Encounters|GetControl%20Points)))
  (bind _output_get (LocalVariables|SetTemp_Control%20Points _keys))
  (if (Utilities|Array|IsValidIndex _output_get) ; Check Control points have been used
    (if _returnvalue
      (bind _output_get_2 (LocalVariables|SetTemp_Current%20Control%20Point _value))
      (Utilities|Array|RemoveItem _output_get _output_get_2) ; Removes currently assigned control point before running checks
    )
    (Utilities|FlowControl|Sequence
      (:then_0
        ;[1 1 1] Find a new Control Point
        (Utilities|FlowControl|ForLoopwithBreak 0 (* (Utilities|Array|LastIndex (LocalVariables|GetTemp_Control%20Points)) 2) :!label _label
          (:LoopBody
            (LocalVariables|SetTemp_Int (Math|Random|RandomInteger (Utilities|Array|Length (LocalVariables|GetTemp_Control%20Points))))
            (if (> (.Value (Utilities|Map|Find (Variables|RebelX|CombatManager|Encounters|GetControl%20Points) (Utilities|Array|Get(acopy) (LocalVariables|GetTemp_Control%20Points) (LocalVariables|GetTemp_Int)))) 0)
              (LocalVariables|SetTemp_New%20Control%20Point%20Index (LocalVariables|GetTemp_Int))
              (LocalVariables|SetControl%20Point%20Found true)
              (goto _label Break)))))
      (:then_1
        (if (LocalVariables|GetControl%20Point%20Found)
          (return true (Utilities|Array|Get(acopy) (LocalVariables|GetTemp_Control%20Points) (LocalVariables|GetTemp_New%20Control%20Point%20Index)))
          (else
            (return false 0)))))
    (else
      (return false 0))))

(fn ReturnAttackTokens
  (params (Attack%20Tokens :type Integer))
  (bind _output_get (Variables|RebelX|CombatManager|SetAvalible%20Attack%20Tokens (+ Attack%20Tokens (Variables|RebelX|CombatManager|GetAvalible%20Attack%20Tokens))))
  (CallFunction|DebugLog (Utilities|String|Append "Attack Tokens: " (Utilities|String|ToString(Integer) _output_get)) "NewEnumerator0" "Attack Tokens" (Variables|RebelX|GetDebug))
  (return true))