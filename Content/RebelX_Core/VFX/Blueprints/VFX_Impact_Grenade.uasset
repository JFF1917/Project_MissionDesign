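; Grenade explosion impact effect that supplies surface-specific visuals and a sound to its parent impact VFX class through asset getter overrides.
; GetSystemAsset selects a Niagara explosion by SurfaceType, with dedicated variants for several materials, a generic one for most others and an air burst for Default and Blood.
; GetAudioAsset returns one explosion sound for all surfaces, while GetDecalAsset defers to the parent.
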(event EventBeginPlay
  (|CallParentFunction) ; This node is disabled and will not be called.\nDrag off pins to build functionality.
)

(event Collision|EventActorBeginOverlap
  (params (OtherActor :type Actor%20Object%20Reference))
  (|CallParentFunction OtherActor) ; This node is disabled and will not be called.\nDrag off pins to build functionality.
)

(event EventTick
  (params (DeltaSeconds :type Float%20%28single-precision%29))
  (|CallParentFunction DeltaSeconds) ; This node is disabled and will not be called.\nDrag off pins to build functionality.
)

(fn ConstructionScript
  (|CallParentFunction))

(fn GetAudioAsset
  (return "/Game/RebelX_Core/Audio/Explosions/SC_Grenade_Explode.SC_Grenade_Explode"))

(fn GetDecalAsset
  (bind _returnvalue (|CallParentFunction))
  (return _returnvalue))

(fn GetSystemAsset
  (return (Utilities|Select :Index (Variables|Default|GetSurfaceType) :SurfaceType_Default "/Game/RebelX_Core/VFX/Explosions/Systems/NS_Explosion_Air.NS_Explosion_Air" :SurfaceType1 "/Game/RebelX_Core/VFX/Explosions/Systems/NS_Explosion_Default.NS_Explosion_Default" :SurfaceType2 "/Game/RebelX_Core/VFX/Explosions/Systems/NS_Explosion_Air.NS_Explosion_Air" :SurfaceType3 "/Game/RebelX_Core/VFX/Explosions/Systems/NS_Explosion_Default.NS_Explosion_Default" :SurfaceType4 "/Game/RebelX_Core/VFX/Explosions/Systems/NS_Explosion_Default.NS_Explosion_Default" :SurfaceType5 "/Game/RebelX_Core/VFX/Explosions/Systems/NS_Explosion_Default.NS_Explosion_Default" :SurfaceType6 "/Game/RebelX_Core/VFX/Explosions/Systems/NS_Explosion_Default.NS_Explosion_Default" :SurfaceType7 "/Game/RebelX_Core/VFX/Explosions/Systems/NS_Explosion_Concrete.NS_Explosion_Concrete" :SurfaceType8 "/Game/RebelX_Core/VFX/Explosions/Systems/NS_Explosion_Dirt.NS_Explosion_Dirt" :SurfaceType9 "/Game/RebelX_Core/VFX/Explosions/Systems/NS_Explosion_Default.NS_Explosion_Default" :SurfaceType10 "/Game/RebelX_Core/VFX/Explosions/Systems/NS_Explosion_Default.NS_Explosion_Default" :SurfaceType11 "/Game/RebelX_Core/VFX/Explosions/Systems/NS_Explosion_Grass.NS_Explosion_Grass" :SurfaceType12 "/Game/RebelX_Core/VFX/Explosions/Systems/NS_Explosion_Ice.NS_Explosion_Ice" :SurfaceType13 "/Game/RebelX_Core/VFX/Explosions/Systems/NS_Explosion_Grass.NS_Explosion_Grass" :SurfaceType14 "/Game/RebelX_Core/VFX/Explosions/Systems/NS_Explosion_Metal.NS_Explosion_Metal" :SurfaceType15 "/Game/RebelX_Core/VFX/Explosions/Systems/NS_Explosion_Default.NS_Explosion_Default" :SurfaceType16 "/Game/RebelX_Core/VFX/Explosions/Systems/NS_Explosion_Default.NS_Explosion_Default" :SurfaceType17 "/Game/RebelX_Core/VFX/Explosions/Systems/NS_Explosion_Default.NS_Explosion_Default" :SurfaceType18 "/Game/RebelX_Core/VFX/Explosions/Systems/NS_Explosion_Default.NS_Explosion_Default" :SurfaceType19 "/Game/RebelX_Core/VFX/Explosions/Systems/NS_Explosion_Sand.NS_Explosion_Sand" :SurfaceType20 "/Game/RebelX_Core/VFX/Explosions/Systems/NS_Explosion_Snow.NS_Explosion_Snow" :SurfaceType21 "/Game/RebelX_Core/VFX/Explosions/Systems/NS_Explosion_Default.NS_Explosion_Default" :SurfaceType22 "/Game/RebelX_Core/VFX/Explosions/Systems/NS_Explosion_Water.NS_Explosion_Water" :SurfaceType23 "/Game/RebelX_Core/VFX/Explosions/Systems/NS_Explosion_Wood.NS_Explosion_Wood" :SurfaceType24 "/Game/RebelX_Core/VFX/Explosions/Systems/NS_Explosion_Default.NS_Explosion_Default")))