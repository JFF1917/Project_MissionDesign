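; Anim notify that throws a grenade by spawning BP_Throwable_Master at the mesh's Socket_Knife when the animation reaches it.
; Aim comes from the owner's camera rotation via an interface message, falling back to the actor's right vector without a valid camera.
; Cook duration and detonation time are queried from the owner and passed to the throwable, with the owning character as reference and instigator.
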(fn ReceivedNotify
  (params (MeshComp :type Skeletal%20Mesh%20Component%20Object%20Reference) (Animation :type Anim%20Sequence%20Base%20Object%20Reference) (EventReference :type Anim%20Notify%20Event%20Reference%20Structure%20%28by%20ref%29))
  (bind _returnvalue (Components|GetOwner MeshComp))
  (bind _returnvalue_2 (Components|GetOwner MeshComp))
  (bind _ascharacter (Utilities|Casting|CastToCharacter _returnvalue))
  (bind _returnvalue_3 (Class|BPILPAMGPCH|LPAMG-GetCameraComponent(Message) _returnvalue_2))
  (bind (_cook_duration _detonation_time) (Class|BPILPAMGPCH|GetGrenadeCookDuration(Message) (Components|GetOwner MeshComp)))
  (Game|SpawnActorfromClass "/Game/RebelX_Core/Blueprints/Throwables/BP_Throwable_Master.BP_Throwable_Master_C" (Math|Transform|MakeTransform (Transformation|GetSocketLocation MeshComp "Socket_Knife") (select (Utilities|IsValid _returnvalue_3) (Transformation|GetWorldRotation _returnvalue_3) (Math|Conversions|RotationFromXVector (Transformation|GetActorRightVector _returnvalue_2)))) "AlwaysSpawn" "OverrideRootScale" _returnvalue _ascharacter _cook_duration _detonation_time _ascharacter)
  (return true))