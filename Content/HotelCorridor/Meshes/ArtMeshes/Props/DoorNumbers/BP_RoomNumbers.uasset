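; BP_RoomNumbers is a hotel corridor door number prop that displays a three-digit room number using static meshes.
; The construction script converts three per-digit choices to indices into the LVUnits mesh array and sets the Units, Tens and Hundreds components.
; The outer choices are crossed: HundresChoice drives the Units component and UnitChoice drives Hundreds.
; The event graph holds only disabled placeholder events, so there is no runtime logic.
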(event EventBeginPlay)

(event Collision|EventActorBeginOverlap
  (params (OtherActor :type Actor%20Object%20Reference)))

(event EventTick
  (params (DeltaSeconds :type Float%20%28single-precision%29)))

(fn ConstructionScript
  (Components|StaticMesh|SetStaticMesh (Variables|Default|GetUnits) (Utilities|Array|Get(acopy) (LocalVariables|GetLVUnits) (Math|Conversions|ToInteger(Byte) (Variables|Default|GetHundres_Choice))))
  (Components|StaticMesh|SetStaticMesh (Variables|Default|GetTens) (Utilities|Array|Get(acopy) (LocalVariables|GetLVUnits) (Math|Conversions|ToInteger(Byte) (Variables|Default|GetTens_Choice))))
  (Components|StaticMesh|SetStaticMesh (Variables|Default|GetHundreds) (Utilities|Array|Get(acopy) (LocalVariables|GetLVUnits) (Math|Conversions|ToInteger(Byte) (Variables|Default|GetUnit_Choice)))))