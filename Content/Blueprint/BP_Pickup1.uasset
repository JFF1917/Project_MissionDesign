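; Pickup actor that shows an on-screen widget to Player_RebelX and can be removed through interaction.
; Sphere overlap adds WB_Pick1 to the viewport on entry and removes it on exit.
; Interact destroys the actor and, if the player pawn is Player_RebelX, returns the Pocker static mesh; a separate Destroy event removes the actor after a short delay.
; An unconnected chain for a timed WBP_Ps widget and unpause never runs.
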(event OnComponentBeginOverlap(Sphere)
  (params (OverlappedComponent :type Primitive%20Component%20Object%20Reference) (OtherActor :type Actor%20Object%20Reference) (OtherComp :type Primitive%20Component%20Object%20Reference) (OtherBodyIndex :type Integer) (bFromSweep :type Boolean) (SweepResult :type Hit%20Result%20Structure%20%28by%20ref%29))
  (Utilities|Casting|CastToPlayer_RebelX OtherActor)
  (bind _returnvalue (UserInterface|CreateWidget "/Game/Blueprint/WB_Pick1.WB_Pick1_C"))
  (UserInterface|Viewport|AddtoViewport _returnvalue 0))

(event OnComponentEndOverlap(Sphere)
  (params (OverlappedComponent :type Primitive%20Component%20Object%20Reference) (OtherActor :type Actor%20Object%20Reference) (OtherComp :type Primitive%20Component%20Object%20Reference) (OtherBodyIndex :type Integer))
  (Utilities|Casting|CastToPlayer_RebelX OtherActor)
  (Widget|RemovefromParent (stale OnComponentBeginOverlap(Sphere) _returnvalue)))

(event Custom|Destroy
  (Utilities|FlowControl|Delay 0.2)
  (Actor|DestroyActor))

(event EventBeginPlay)

(event EventTick
  (params (DeltaSeconds :type Float%20%28single-precision%29)))

(fn ConstructionScript)

(fn Interact
  (Actor|DestroyActor)
  (Utilities|Casting|CastToPlayer_RebelX (Game|Player|GetPlayerPawn 0))
  (return (Variables|/Script/Engine.StaticMeshComponent|GetStaticMesh (Variables|Default|GetPocker))))