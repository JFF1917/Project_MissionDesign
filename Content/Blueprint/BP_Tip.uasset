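; BP_Tip is a one-time trigger box that shows a dialogue tip when the Player_RebelX character enters it.
; Begin overlap creates a WBP_Chat widget and plays the Dialogue_20001 2D sound through a DoOnce.
; After a fixed delay it unpauses the game, though this graph never pauses it, and removes the widget.
; End overlap also removes the widget through its own DoOnce, so leaving early closes the tip.
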(event OnComponentBeginOverlap(Box)
  (params (OverlappedComponent :type Primitive%20Component%20Object%20Reference) (OtherActor :type Actor%20Object%20Reference) (OtherComp :type Primitive%20Component%20Object%20Reference) (OtherBodyIndex :type Integer) (bFromSweep :type Boolean) (SweepResult :type Hit%20Result%20Structure%20%28by%20ref%29))
  (Utilities|Casting|CastToPlayer_RebelX OtherActor)
  (Utilities|FlowControl|DoOnce false
    (:Completed
      (bind _returnvalue (UserInterface|CreateWidget "/Game/Blueprint/WBP_Chat.WBP_Chat_C"))
      (UserInterface|Viewport|AddtoViewport _returnvalue 0)
      (Audio|PlaySound2D "/Game/Audio/Dialogue_20001.Dialogue_20001" 1.0 1.0 0.0 0 0)
      (Utilities|FlowControl|Delay 25.0)
      (Game|SetGamePaused false)
      (Widget|RemovefromParent _returnvalue))))

(event OnComponentEndOverlap(Box)
  (params (OverlappedComponent :type Primitive%20Component%20Object%20Reference) (OtherActor :type Actor%20Object%20Reference) (OtherComp :type Primitive%20Component%20Object%20Reference) (OtherBodyIndex :type Integer))
  (Utilities|Casting|CastToPlayer_RebelX OtherActor)
  (Utilities|FlowControl|DoOnce false
    (:Completed
      (Widget|RemovefromParent (stale OnComponentBeginOverlap(Box) _returnvalue)))))

(event EventBeginPlay)

(event Collision|EventActorBeginOverlap
  (params (OtherActor :type Actor%20Object%20Reference)))

(event EventTick
  (params (DeltaSeconds :type Float%20%28single-precision%29)))

(fn ConstructionScript)